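; BP_XML_Template is an example Blueprint that builds and saves an XML document on BeginPlay.
; It creates a document with a comment, a Products root and a Users element, then adds a Company element and user entries with map-based credential attributes.
; Success checks on most element additions gate the save to a hard-coded local Downloads path.
; A document print-to-screen branch is present but unwired.
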(event `self.ReceiveBeginPlay`
  (bind _out_doc (`FF_XMLBPLibrary.XML_Doc_Create` ""))
  (bind _output_get (set `self.REF_XML` _out_doc))
  (`FF_XMLBPLibrary.XML_Comment_Add` _output_get "Product attributes.")
  (bind _out_element (`FF_XMLBPLibrary.XML_Element_Add_Single` (`self.REF_XML`) "Products"))
  (bind _output_get_2 (set `self.REF_Element_Root` _out_element))
  (bind (_out_element_2 _returnvalue) (`FF_XMLBPLibrary.XML_Element_Add_Single` _output_get_2 "Users"))
  (if _returnvalue
    (set `self.REF_Element_Users` _out_element_2)
    (bind (_out_element_3 _returnvalue_2) (`FF_XMLBPLibrary.XML_Element_Add_Single` (`self.REF_Element_Users`) "Company" "Frozen Forest"))
    (if _returnvalue_2
      (bind (_out_element_4 _returnvalue_3) (`FF_XMLBPLibrary.XML_Element_Add_Map` (`self.REF_Element_Users`) "user" "Luffy" (`|MakeMap` "username" "Eray" "password" "123456")))
      (if _returnvalue_3
        (bind (_out_element_5 _returnvalue_4) (`FF_XMLBPLibrary.XML_Element_Add_Map` (`self.REF_Element_Users`) "user" "Usoop" (`|MakeMap` "username" "Mustafa" "password" "789")))
        (if _returnvalue_4
          (`FF_XMLBPLibrary.XML_Doc_Save` (`self.REF_XML`) "C:\\Users\\erayo\\Downloads\\test.xml"))))))

(fn `UserConstructionScript`)