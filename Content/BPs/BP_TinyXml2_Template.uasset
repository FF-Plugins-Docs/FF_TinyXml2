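; Template Blueprint demonstrating a TinyXML2 plugin's XML document functions.
; On BeginPlay it opens an XML file from a hardcoded local path and prints its contents on screen.
; Unwired chains build a document with comment, elements and attribute maps, print it between timed element and comment removals, and save to disk.
; A Samples graph holds unconnected example nodes for the library calls.
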(event `self.ReceiveBeginPlay`
  (bind (_out_doc _returnvalue) (`FF_TinyXml2BPLibrary.TinyXML2_Open_File` "C:\\Users\\erayo\\Downloads\\sample3.xml"))
  (if _returnvalue
    (bind _out_string (`FF_TinyXml2BPLibrary.TinyXML2_Doc_Print` _out_doc))
    (`KismetSystemLibrary.PrintString` _out_string true true (struct :`G` 0.66 :`B` 1.0 :`A` 1.0) 60.0)))

(fn `UserConstructionScript`)